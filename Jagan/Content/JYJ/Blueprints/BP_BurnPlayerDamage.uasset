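; BP_BurnPlayerDamage is a floating text actor that displays the burn status label "화상" (Burn).
; On BeginPlay it stores its location, then a Timeline vector track offsets the TextRender's height with Z and drives its X/Y scale with Y.
; The actor destroys itself when the Timeline finishes.
; SetDamageText writes the fixed label and is not called within this Blueprint.
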(event `self.ReceiveBeginPlay`
  (bind _textrender (`self.TextRender`))
  (set `self.DamagePos` (`self.K2_GetActorLocation`))
  (bind (_direction _newtrack_0) (`Timeline|Timeline`)
    (:`Update`
      (bind _y (.y _newtrack_0))
      (`SceneComponent.K2_SetWorldLocation` (`self.TextRender`) (+ (`self.DamagePos`) (`KismetMathLibrary.MakeVector` 0.0 0.0 (.z _newtrack_0))) false false)
      (`TextRenderComponent.SetXScale` _textrender _y)
      (`TextRenderComponent.SetYScale` _textrender _y))
    (:`Finished`
      (`self.K2_DestroyActor`))))

(fn `SetDamageText`
  (`TextRenderComponent.K2_SetText` (`self.TextRender`) (`KismetTextLibrary.Conv_StringToText` "화상")))

(fn `UserConstructionScript`)