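; BP_BossCam is the boss-fight dungeon camera, rising into position and then following the player.
; BeginPlay caches the BP_Player actor as its target.
; After the AutoCameraMove delay, Tick nudges the camera along X and Z by a fixed per-frame step.
; Past a height threshold, it pins X and Z and tracks only the player's Y, with a small delta-time-scaled offset.
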(event `self.ReceiveActorBeginOverlap`
  (params (OtherActor :type "Actor Object Reference")))

(event `self.ReceiveBeginPlay`
  ;[1 1 1] 던전캠 시작할 때, 카메라 타겟팅
  (bind _returnvalue (`GameplayStatics.GetActorOfClass` "/Game/JYJ/Blueprints/BP_Player.BP_Player_C"))
  (set `self.Target` _returnvalue))

(event `self.ReceiveTick`
  (params (DeltaSeconds :type "Float (single-precision)"))
  (bind (_returnvalue_x _returnvalue_y _returnvalue_z) (`KismetMathLibrary.BreakVector` (`self.K2_GetActorLocation`)))
  (bind (_returnvalue_x_2 _returnvalue_y_2 _returnvalue_z_2) (`KismetMathLibrary.BreakVector` (`self.K2_GetActorLocation`)))
  (bind (_returnvalue_x_3 _returnvalue_y_3 _returnvalue_z_3) (`KismetMathLibrary.BreakVector` (`self.K2_GetActorLocation`)))
  (bind (_returnvalue_x_4 _returnvalue_y_4) (`KismetMathLibrary.BreakVector` (`self.K2_GetActorLocation`)))
  (bind (_returnvalue_x_5 _returnvalue_y_5) (`KismetMathLibrary.BreakVector` (`self.K2_GetActorLocation` (`self.Target`))))
  (bind (_returnvalue_x_6 _returnvalue_y_6) (`KismetMathLibrary.BreakVector` (`self.K2_GetActorLocation` (`self.Target`))))
  ;[1 1 1] 캐릭터 카메라 위치 가져와서 특정 위치 도달까지 x, z좌표 +3, 상한선 도달 시,  y축만 움직임
  (set `self.CurrentTime` (+ (`self.CurrentTime`) (`GameplayStatics.GetWorldDeltaSeconds`)))
  (if (and (>= (`self.CurrentTime`) (`self.AutoCameraMove`)) (<= _returnvalue_z_2 1175.0))
    (`KismetSystemLibrary.PrintString` (`KismetStringLibrary.Conv_VectorToString` (`self.K2_GetActorLocation`)))
    (`self.K2_SetActorLocation` (`KismetMathLibrary.MakeVector` (+ _returnvalue_x 3.0) _returnvalue_y (+ _returnvalue_z 3.0)))
    (if (>= _returnvalue_z_3 1100.0)
      ;[1 1 1] 보스 전투맵, y축만 플레이어 따라가기
      (`self.K2_SetActorLocation` (`KismetMathLibrary.MakeVector` -1360.0 (+ _returnvalue_y_5 (* (- _returnvalue_y_6 _returnvalue_y_4) (`GameplayStatics.GetWorldDeltaSeconds`) 1.0)) 1175.0)))))

(fn `UserConstructionScript`)