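; Game mode Blueprint, named for player movement, that sets up the HUD and shows boss-death and game-clear screen widgets.
; On BeginPlay it adds player and boss HP widgets, unpauses, and sets game-only input, immediately overridden by game-and-UI input.
; Custom events add a work-info text widget after boss death and a fade-out on game clear, with debug prints.
; The work-info widget's removal node is unconnected.
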(event `self.ReceiveBeginPlay`
  (bind _returnvalue (`GameplayStatics.GetPlayerController` 0))
  (`|ExecutionSequence`
    (:`then_0`
      (bind _returnvalue_2 (`|CreateWidget` "/Game/JYJ/Blueprints/UI/WBP_PlayerHP.WBP_PlayerHP_C"))
      (`UserWidget.AddToViewport` _returnvalue_2 0))
    (:`then_1`
      (bind _returnvalue_3 (`|CreateWidget` "/Game/KSH/UI/WBP_BossHP.WBP_BossHP_C"))
      (`UserWidget.AddToViewport` _returnvalue_3 0))
    (:`then_2`
      (`WidgetBlueprintLibrary.SetInputMode_GameOnly` _returnvalue)
      (`GameplayStatics.SetGamePaused` false))
    (:`then_3`
      (`WidgetBlueprintLibrary.SetInputMode_GameAndUIEx` _returnvalue null))))

(event `BossDieWallControlInfo`
  (bind _returnvalue (`|CreateWidget` "/Game/KSH/UI/WBP_WorkInfoText.WBP_WorkInfoText_C"))
  (`UserWidget.AddToViewport` _returnvalue 0)
  (`KismetSystemLibrary.Delay` 1.0)
  (`KismetSystemLibrary.PrintString` (`KismetSystemLibrary.GetDisplayName` _returnvalue)))

(event `GameClear_FadeOut`
  ;[1 1 1] FadeOut 시작
  (`KismetSystemLibrary.Delay` 0.1)
  (bind _returnvalue (`|CreateWidget` "/Game/KSH/UI/WBP_FadeOut.WBP_FadeOut_C"))
  (`UserWidget.AddToViewport` _returnvalue 1)
  (`/Game/KSH/UI/WBP_FadeOut.FadeOutEvent` _returnvalue)
  (`KismetSystemLibrary.PrintString` "GameClear"))

(fn `UserConstructionScript`)