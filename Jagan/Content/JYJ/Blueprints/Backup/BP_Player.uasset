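; Player character with mouse-aimed basic magic, four spawned skills, a cursor-directed launch dash and wall interaction.
; Spells spawn actors and deduct their MP cost; only Wind checks MP first, and it also zeroes HP.
; Tick regenerates HP and MP through a shared timer and pauses into a game-over widget at zero HP.
; Includes damage-over-time handling and debug inputs for boss damage and phase.
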(event `self.ReceiveTick`
  (params (DeltaSeconds :type "Float (single-precision)"))
  ;[1 1 1] HP, MP 자동회복 / HP = 0 일 때, 사망처리
  (`|ExecutionSequence`
    (:`then_0`
      (`self.PlayerDie`))
    (:`then_1`
      (`self.PlayerRestoreMP`))
    (:`then_2`
      (`self.PlayerRestoreHP`))))

(event `self.ReceiveBeginPlay`
  ;[1 1 1] Player HP,  MP SETTING
  (set `self.HP` (`self.MaxHP`))
  (set `self.MP` (`self.MaxMP`))
  (bind _returnvalue (`GameplayStatics.GetActorOfClass` "/Game/KSH/Blueprints/BP_Boss.BP_Boss_C"))
  (set `self.BP_Boss` _returnvalue))

(event `InputAxisKey|MouseWheelAxis`
  (params (AxisValue :type "Float (single-precision)"))
  (bind _springarm (`self.SpringArm`))
  (set `SpringArmComponent.TargetArmLength` (+ (* AxisValue -100.0) (`SpringArmComponent.TargetArmLength` _springarm)) _springarm))

(event `InputAction|AttackPlayer`
  (params (Key :type "Key Structure"))
  ;[1 1 1] 좌클릭 시, 기본 공격
  (:`Pressed`
    (if (not (`self.IsAttackLeftMouse`))
      (set `self.IsAttackLeftMouse` true)
      (`KismetSystemLibrary.PrintString` "공격!" true true (struct :`R` 1.0 :`G` 0.048188 :`A` 1.0))
      (`self.AttackBasic`)))
  (:`Released`
    (set `self.IsAttackLeftMouse` false)))

(event `SkillWind`
  (bind (_returnvalue_location _returnvalue_rotation) (`KismetMathLibrary.BreakTransform` (`SceneComponent.K2_GetComponentToWorld` (`self.Arrow1`))))
  ;[1 1 1] 돌풍 스킬 소환
  (bind _returnvalue (`|SpawnActorFromClass` "/Game/JYJ/Blueprints/Skill/BP_SkillWind.BP_SkillWind_C" (`KismetMathLibrary.MakeTransform` _returnvalue_location _returnvalue_rotation) "Undefined" "MultiplyWithRoot" null null))
  (bind _output_get (set `self.MP` (- (`self.MP`) (`/Game/JYJ/Blueprints/Skill/BP_SkillWind.UseMP` _returnvalue))))
  (`KismetSystemLibrary.PrintString` (`KismetStringLibrary.Conv_IntToString` _output_get)))

(event `AttackBasic`
  ;[1 1 1] 기본 마법 공격 소환
  (`|ExecutionSequence`
    (:`then_0`
      (bind (_direction _rotation) (`self.SkillSpawnDirection`))
      (`self.K2_SetActorRotation` _rotation))
    (:`then_1`
      (`self.PlayAnimMontage` "/Game/JYJ/Blueprints/Animation/AMP_PlayerBasicSkill.AMP_PlayerBasicSkill"))
    (:`then_2`
      (bind _returnvalue (`|SpawnActorFromClass` "/Game/JYJ/Blueprints/Skill/SkillBasic/BP_SkillBasic.BP_SkillBasic_C" (`KismetMathLibrary.MakeTransform` _direction _rotation) "Undefined" "MultiplyWithRoot" null null))
      (bind _output_get (set `self.MP` (- (`self.MP`) (`/Game/JYJ/Blueprints/Skill/SkillBasic/BP_SkillBasic.UseMP` _returnvalue))))
      (`KismetSystemLibrary.PrintString` (`KismetStringLibrary.Conv_IntToString` _output_get)))))

(event `InputAction|Skill_Wind`
  (params (Key :type "Key Structure"))
  ;[1 1 1] 스킬_돌풍
  (:`Pressed`
    (if (< (`self.MP`) (`self.SkillWindMP`))
      (`KismetSystemLibrary.PrintString` "스킬 사용 불가능" true true (struct :`R` 1.0 :`B` 0.117779 :`A` 1.0))
      (else
        (`KismetSystemLibrary.PrintString` "돌풍!" true true (struct :`R` 0.184767 :`G` 0.859986 :`B` 1.0 :`A` 1.0))
        (`self.SkillWind`)
        (set `self.HP` 0)))))

(event `InputAction|BossHPDecreaseTest`
  (params (Key :type "Key Structure"))
  ;[1 1 1] BOSS 데미지, 페이즈 전환 TEST
  (:`Pressed`
    (bind _resulthp (`/Game/KSH/Blueprints/BP_Boss.BossApplyDamage` (`self.BP_Boss`) 50))
    (if (<= _resulthp 0)
      (`/Game/KSH/Blueprints/BP_Boss.BossDieEvent` (`self.BP_Boss`)))))

(event `SkillElem`
  (bind (_returnvalue_location _returnvalue_rotation) (`KismetMathLibrary.BreakTransform` (`SceneComponent.K2_GetComponentToWorld` (`self.Arrow1`))))
  ;[1 1 1] 엘리멘탈 스킬 소환
  (bind _returnvalue (`|SpawnActorFromClass` "/Game/JYJ/Blueprints/Skill/BP_SkillElem.BP_SkillElem_C" (`KismetMathLibrary.MakeTransform` _returnvalue_location _returnvalue_rotation) "Undefined" "MultiplyWithRoot" null null))
  (bind _output_get (set `self.MP` (- (`self.MP`) (`/Game/JYJ/Blueprints/Skill/BP_SkillElem.UseMP` _returnvalue))))
  (`KismetSystemLibrary.PrintString` (`KismetStringLibrary.Conv_IntToString` _output_get)))

(event `InputAction|Dash`
  (params (Key :type "Key Structure"))
  (bind _returnvalue (`KismetMathLibrary.Normal` (- (`.ImpactPoint` (`GameplayStatics.BreakHitResult` (`PlayerController.GetHitResultUnderCursorByChannel` (`GameplayStatics.GetPlayerController` 0) "TraceTypeQuery1" true))) (`self.K2_GetActorLocation`))))
  ;[1 1 1] SPACE 회피기
  (:`Pressed`
    (`GameplayStatics.SpawnEmitterAtLocation` "/Game/JYJ/Blueprints/Move/P_WingBlast.P_WingBlast" (`self.K2_GetActorLocation`) (struct) (0.5 0.5 0.5) false)
    (`self.LaunchCharacter` (* _returnvalue 7000.0))
    (`self.K2_SetActorRotation` (`KismetMathLibrary.MakeRotFromXZ` _returnvalue (`self.GetActorUpVector`)))
    (`KismetSystemLibrary.Delay` 0.2)
    (`GameplayStatics.SpawnEmitterAtLocation` "/Game/JYJ/Blueprints/Move/P_WingBlast.P_WingBlast" (`self.K2_GetActorLocation`) (struct) (0.5 0.5 0.5) false)))

(event `Key|One`
  (params (Key :type "Key Structure"))
  ;[1 1 1] BOSS 데미지, 페이즈 전환 TEST
  (:`Pressed`
    (set `/Game/KSH/Blueprints/BP_Boss.Phase` 1 (`self.BP_Boss`))))

(event `Key|Zero`
  (params (Key :type "Key Structure"))
  ;[1 1 1] BOSS 데미지, 페이즈 전환 TEST
  (:`Pressed`
    (set `/Game/KSH/Blueprints/BP_Boss.Phase` 0 (`self.BP_Boss`))))

(event `InputAction|Skill_Element`
  (params (Key :type "Key Structure"))
  ;[1 1 1] 스킬_엘리멘탈
  (:`Pressed`
    (`KismetSystemLibrary.PrintString` "엘리멘탈!" true true (struct :`R` 0.827089 :`G` 0.005004 :`B` 1.0 :`A` 1.0))
    (`self.SkillElem`)))

(event `PlayerApplyDotDamageEvent`
  (params (DamageDuration :type Integer) (Damage :type Integer))
  ;[1 1 1] 화상 데미지 이벤트
  (bind _counter (`/Engine/EditorBlueprintResources/StandardMacros.Do N` DamageDuration :!label _label)
    (:`Exit`
      (`self.PlayerApplyDamage` Damage)
      (`KismetSystemLibrary.Delay` 0.5)
      (if (not (>= _counter DamageDuration))
        (goto _label)))))

(event `SkillFire`
  (bind (_returnvalue_location _returnvalue_rotation) (`KismetMathLibrary.BreakTransform` (`SceneComponent.K2_GetComponentToWorld` (`self.Arrow1`))))
  ;[1 1 1] 종말의 날 스킬 소환
  (bind _returnvalue (`|SpawnActorFromClass` "/Game/JYJ/Blueprints/Skill/BP_SkillFire.BP_SkillFire_C" (`KismetMathLibrary.MakeTransform` _returnvalue_location _returnvalue_rotation) "Undefined" "MultiplyWithRoot" null null))
  (bind _output_get (set `self.MP` (- (`self.MP`) (`/Game/JYJ/Blueprints/Skill/BP_SkillFire.UseMP` _returnvalue))))
  (`KismetSystemLibrary.PrintString` (`KismetStringLibrary.Conv_IntToString` _output_get)))

(event `InputAction|Skill_Fire`
  (params (Key :type "Key Structure"))
  ;[1 1 1] 스킬_종말의 날
  (:`Pressed`
    (`KismetSystemLibrary.PrintString` "종말의 날!" true true (struct :`R` 1.0 :`B` 0.041135 :`A` 1.0))
    (`self.SkillFire`)))

(event `SkillIce`
  (bind (_returnvalue_location _returnvalue_rotation) (`KismetMathLibrary.BreakTransform` (`SceneComponent.K2_GetComponentToWorld` (`self.Arrow1`))))
  ;[1 1 1] 아이스에로우 스킬 소환
  (bind _returnvalue (`|SpawnActorFromClass` "/Game/JYJ/Blueprints/Skill/SkillIce/BP_SkillIce.BP_SkillIce_C" (`KismetMathLibrary.MakeTransform` _returnvalue_location _returnvalue_rotation) "Undefined" "MultiplyWithRoot" null null))
  (bind _output_get (set `self.MP` (- (`self.MP`) (`/Game/JYJ/Blueprints/Skill/SkillIce/BP_SkillIce.UseMP` _returnvalue))))
  (`KismetSystemLibrary.PrintString` (`KismetStringLibrary.Conv_IntToString` _output_get)))

(event `InputAction|Skill_Ice`
  (params (Key :type "Key Structure"))
  ;[1 1 1] 스킬_아이스에로우
  (:`Pressed`
    (`KismetSystemLibrary.PrintString` "아이스!" true true (struct :`R` 1.0 :`G` 1.0 :`B` 1.0 :`A` 1.0))
    (`self.SkillIce`)))

(event `Key|G`
  (params (Key :type "Key Structure"))
  ;[1 1 1] 범위에 있으면 상호작용 가능
  (:`Pressed`
    (bind (_outactors _returnvalue) (`KismetSystemLibrary.SphereOverlapActors` (`self.K2_GetActorLocation`) 200.0 (`|MakeArray` "ObjectTypeQuery2" :!type "EObjectTypeQuery Enum") "/Game/KSH/Blueprints/BP_WallController.BP_WallController_C"))
    (if _returnvalue
      (for _array_element _outactors
        (bind _asbp_wall_controller (cast `/Game/KSH/Blueprints/BP_WallController` _array_element))
        (`/Game/KSH/Blueprints/BP_WallController.OpenWall` _asbp_wall_controller)))))

(event `self.ReceiveActorBeginOverlap`
  (params (OtherActor :type "Actor Object Reference"))
  ;[1 1 1] 장판 맞으면 맞은 장판 이름 화면에 표시
)

(fn `PlayerApplyDamage`
  (params (Damage :type Integer))
  (returns (ResultHP :type Integer))
  (bind _output_get (set `self.HP` (- (`self.HP`) Damage)))
  (return _output_get))

(fn `PlayerDie`
  (if (<= (`self.HP`) 0)
    (bind _returnvalue (`|CreateWidget` "/Game/JYJ/Blueprints/UI/WBP_PlayerGameOver.WBP_PlayerGameOver_C"))
    (`UserWidget.AddToViewport` _returnvalue 0)
    (`WidgetBlueprintLibrary.SetInputMode_UIOnlyEx` (`GameplayStatics.GetPlayerController` 0) null)
    (`GameplayStatics.SetGamePaused` true)))

(fn `PlayerRestoreHP`
  (if (< (`self.HP`) (`self.MaxHP`))
    (set `self.CurrentTime` (+ (`self.CurrentTime`) (`GameplayStatics.GetWorldDeltaSeconds`)))
    (if (>= (`self.CurrentTime`) (`self.AutoRestoreHP`))
      (`/Engine/EditorBlueprintResources/StandardMacros.IncrementInt` (`self.HP`)
        (:`  `
          (set `self.CurrentTime` 0.0))))))

(fn `PlayerRestoreMP`
  (if (< (`self.MP`) (`self.MaxMP`))
    (set `self.CurrentTime` (+ (`self.CurrentTime`) (`GameplayStatics.GetWorldDeltaSeconds`)))
    (if (>= (`self.CurrentTime`) (`self.AutoRestoreMP`))
      (bind _result (`/Engine/EditorBlueprintResources/StandardMacros.IncrementInt` (`self.MP`))
        (:`  `
          (set `self.MP` _result)
          (set `self.CurrentTime` 0.0))))))

(fn `SkillSpawnDirection`
  (returns (Direction :type "Vector Structure") (Rotation :type "Rotator Structure"))
  (bind _returnvalue (`KismetMathLibrary.Normal` (- (`.Location` (`GameplayStatics.BreakHitResult` (`PlayerController.GetHitResultUnderCursorByChannel` (`GameplayStatics.GetPlayerController` 0) "TraceTypeQuery1" true))) (`self.K2_GetActorLocation` (`GameplayStatics.GetPlayerPawn` 0)))))
  (return (+ (`self.K2_GetActorLocation`) (* _returnvalue (`self.Speed`) (`GameplayStatics.GetWorldDeltaSeconds`))) (`KismetMathLibrary.MakeRotFromXZ` _returnvalue (`self.GetActorUpVector` (`GameplayStatics.GetPlayerPawn` 0)))))

(fn `Translate`
  (params (Direction :type "Vector Structure") (Speed :type "Float (double-precision)"))
  ;[1 1 1] P = p0 + velovity(dir*speed)*deltaSecond
  (`self.K2_SetActorLocation` (+ (`self.K2_GetActorLocation`) (* Direction Speed (`GameplayStatics.GetWorldDeltaSeconds`)))))

(fn `UserConstructionScript`)