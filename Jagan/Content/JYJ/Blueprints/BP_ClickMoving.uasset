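; Player controller Blueprint that moves the controlled pawn toward the mouse cursor while the MovingPlayer input (right-click) is held.
; Press and release toggle a flag that Tick checks to trace under the cursor on the Visibility channel.
; Each hit calls SimpleMoveToLocation if over 100 units from the pawn, and spawns a BP_PlayerLocation actor there regardless of distance, every held frame.
; Debug strings print movement and hit location.
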(event `self.ReceiveTick`
  (params (DeltaSeconds :type "Float (single-precision)"))
  ;[1 1 1] IsClickRightMouse에 따라 마우스 커서로 위치 이동
  (if (`self.IsClickRightMouse`)
    (`self.MoveToMouseCursor`)))

(event `InputAction|MovingPlayer`
  (params (Key :type "Key Structure"))
  ;[1 1 1] 우클릭 시, IsClickRightMouse 변수 값 변경
  (:`Pressed`
    (`self.InputRightMouseButtonPress`))
  (:`Released`
    (`self.InputRightMouseButtonRelease`)))

(fn `InputRightMouseButtonPress`
  (set `self.IsClickRightMouse` true))

(fn `InputRightMouseButtonRelease`
  (set `self.IsClickRightMouse` false))

(fn `MoveToMouseCursor`
  (bind (_hitresult _returnvalue) (`self.GetHitResultUnderCursorByChannel` self "TraceTypeQuery1" true))
  (bind (_bblockinghit _binitialoverlap _time _distance _location) (`GameplayStatics.BreakHitResult` _hitresult))
  (if _returnvalue
    (`self.SetNewDestination` _location)
    (`|SpawnActorFromClass` "/Game/JYJ/Blueprints/BP_PlayerLocation.BP_PlayerLocation_C" (`KismetMathLibrary.Conv_VectorToTransform` _location) "Undefined" "MultiplyWithRoot" null null)
    (`KismetSystemLibrary.PrintString` (`KismetStringLibrary.Conv_VectorToString` _location) true true (struct :`A` 1.0))))

(fn `SetNewDestination`
  (params (NewDirection :type "Vector Structure"))
  (if (> (`KismetMathLibrary.Vector_Distance` NewDirection (`self.K2_GetActorLocation` (`self.K2_GetPawn`))) 100.0)
    (`AIBlueprintHelperLibrary.SimpleMoveToLocation` self NewDirection)
    (`KismetSystemLibrary.PrintString` "나는 열심히 움직인다...")))

(fn `UserConstructionScript`)