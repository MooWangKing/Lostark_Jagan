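; BP_SkillBasic is the basic attack projectile used against the boss, built around a Sphere and a ProjectileMovement component.
; On Hit, it casts the other actor to BP_Boss, calls BossApplyDamage with a fixed amount and writes the result to BossHP.
; When the projectile stops, it hides the sphere, attaches a dissolve particle effect and sets a short lifespan.
; Older cursor-following movement, duplicate damage logic and debug prints remain unconnected.
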(event `self.ReceiveTick`
  (params (DeltaSeconds :type "Float (single-precision)")))

(event `self.ReceiveActorBeginOverlap`
  (params (OtherActor :type "Actor Object Reference"))
  ;[1 1 1] 보스 기본 공격 시, 충돌 처리 -> 보스 데미지 함수 호출
)

(event `self.ReceiveHit`
  (params (MyComp :type "PrimitiveComponent Object Reference") (Other :type "Actor Object Reference") (OtherComp :type "PrimitiveComponent Object Reference") (bSelfMoved :type Boolean) (HitLocation :type "Vector Structure") (HitNormal :type "Vector Structure") (NormalImpulse :type "Vector Structure") (Hit :type "HitResult Structure (by ref)"))
  (bind _asbp_boss (cast `/Game/KSH/Blueprints/BP_Boss` Other))
  (bind _resulthp (`/Game/KSH/Blueprints/BP_Boss.BossApplyDamage` _asbp_boss 10))
  (set `/Game/KSH/Blueprints/BP_Boss.BossHP` _resulthp _asbp_boss))

(event `self.ProjectileMovement.OnProjectileStop`
  (params (ImpactResult :type "HitResult Structure (by ref)"))
  (`SceneComponent.SetHiddenInGame` (`self.Sphere`) true false)
  (`self.SetLifeSpan` 1.0)
  (`GameplayStatics.SpawnEmitterAttached` "/Game/JYJ/Blueprints/Skill/P_AngelDissolve.P_AngelDissolve" (`self.Sphere`) "None" (0.0 0.0 0.0) (struct) (3.0 3.0 3.0)))

(fn `UserConstructionScript`)