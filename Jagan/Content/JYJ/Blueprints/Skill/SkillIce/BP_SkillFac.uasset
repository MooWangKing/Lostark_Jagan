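; Ice skill factory actor that spawns a staggered series of BP_SkillIce1 actors at preset points.
; On BeginPlay it gathers eleven spawn-point components into ArrowList and, after a short delay, calls Fire.
; Fire spawns one actor at the current point's world transform, increments FireCount, then calls itself after SpawnTime until the list is exhausted.
; MakeSkill is an empty event.
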(event `Fire`
  (`|SpawnActorFromClass` "/Game/JYJ/Blueprints/Skill/SkillIce/BP_SkillIce1.BP_SkillIce1_C" (`SceneComponent.K2_GetComponentToWorld` (`|GetArrayItem` (`self.ArrowList`) (`self.FireCount`))) "AdjustIfPossibleButAlwaysSpawn" "MultiplyWithRoot" null 1000.0 0.0 null)
  (`KismetSystemLibrary.Delay` 0.2)
  (`/Engine/EditorBlueprintResources/StandardMacros.IncrementInt` (`self.FireCount`)
    (:`  `
      (if (< (`self.FireCount`) (`KismetArrayLibrary.Array_Length` (`self.ArrowList`)))
        (`KismetSystemLibrary.Delay` (`self.SpawnTime`))
        (`self.Fire`)))))

(event `self.ReceiveBeginPlay`
  (set `self.ArrowList` (`|MakeArray` (`self.Spawn`) (`self.Spawn1`) (`self.Spawn2`) (`self.Spawn3`) (`self.Spawn4`) (`self.Spawn5`) (`self.Spawn6`) (`self.Spawn7`) (`self.Spawn8`) (`self.Spawn9`) (`self.Spawn10`)))
  (set `self.FireCount` 0)
  (`KismetSystemLibrary.Delay` 0.5)
  (`self.Fire`))

(event `MakeSkill`)

(fn `UserConstructionScript`)