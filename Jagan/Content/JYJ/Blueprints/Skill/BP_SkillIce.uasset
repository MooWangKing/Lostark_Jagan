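; BP_SkillIce is a projectile actor for an ice skill, noted in its comments as the shot fired by a basic attack.
; Tick moves it along its forward vector at Speed with no sweep, and also sets UseMP to a fixed cost every frame.
; Overlapping a BP_Boss only prints the boss's name; the actor applies no damage and does not destroy itself.
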(event `self.ReceiveTick`
  (params (DeltaSeconds :type "Float (single-precision)"))
  ;[1 1 1] 기본 공격 시, 동그라미 발싸!
  (`self.K2_SetActorLocation` (+ (`self.K2_GetActorLocation`) (* DeltaSeconds (`self.GetActorForwardVector`) (`self.Speed`))))
  (set `self.UseMP` 20))

(event `self.ReceiveBeginPlay`)

(event `self.ReceiveActorBeginOverlap`
  (params (OtherActor :type "Actor Object Reference"))
  ;[1 1 1] 보스 기본 공격 시, 충돌 처리
  (bind _asbp_boss (cast `/Game/KSH/Blueprints/BP_Boss` OtherActor))
  (`KismetSystemLibrary.PrintString` (`KismetSystemLibrary.GetDisplayName` _asbp_boss) true true (struct :`R` 0.328125 :`G` 0.02629 :`B` 0.006836 :`A` 1.0)))

(fn `UserConstructionScript`)