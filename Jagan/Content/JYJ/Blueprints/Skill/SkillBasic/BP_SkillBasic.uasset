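; BP_SkillBasic is a basic skill projectile that damages BP_Boss on hit, writing the boss's HP from BossApplyDamage.
; Half a second after spawn, it bursts and destroys itself if its max speed equals 500.
; When the projectile stops, it hides its sphere, attaches a dissolve effect and expires shortly after.
; Tick spawns non-auto-destroy emitters every frame, adding a second one once elapsed time passes AutoincreaseTime, with debug prints.
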(event `self.ReceiveBeginPlay`
  ;[1 1 1] 발사체 최고 속력일  때, 이펙트 추가
  (`KismetSystemLibrary.K2_SetTimerDelegate` (delegate `OnTimer`) 0.5))

(event `OnTimer`
  ;[1 1 1] 발사체 최고 속력일  때, 이펙트 추가
  (if (== (`MovementComponent.GetMaxSpeed` (`self.ProjectileMovement`)) 500.0)
    (`GameplayStatics.SpawnEmitterAtLocation` "/Game/JYJ/Blueprints/Skill/SkillBasic/P_Test.P_Test" (`SceneComponent.K2_GetComponentLocation` (`self.Sphere`)) (struct) (2.0 2.0 2.0))
    (`MovementComponent.StopMovementImmediately` (`self.ProjectileMovement`))
    (`self.K2_DestroyActor`)))

(event `self.ReceiveActorBeginOverlap`
  (params (OtherActor :type "Actor Object Reference")))

(event `self.ReceiveTick`
  (params (DeltaSeconds :type "Float (single-precision)"))
  (bind _autoincreasetime (`self.AutoincreaseTime`))
  ;[1 1 1] 기본 스킬 나갈 때, 바로 붙는 이펙트
  (bind _returnvalue (`GameplayStatics.SpawnEmitterAtLocation` "/Game/JYJ/Blueprints/Skill/SkillBasic/P_AngelDissolve.P_AngelDissolve" (`self.K2_GetActorLocation`) (struct) (0.0 0.0 0.0) false))
  (set `self.CurrentTime` (+ (`self.CurrentTime`) (`GameplayStatics.GetWorldDeltaSeconds`)))
  (if (>= (`self.CurrentTime`) _autoincreasetime)
    (`KismetSystemLibrary.PrintString` (`KismetStringLibrary.Conv_DoubleToString` _autoincreasetime))
    (bind _returnvalue_2 (`GameplayStatics.SpawnEmitterAtLocation` "/Game/JYJ/Blueprints/Skill/SkillBasic/P_Test.P_Test" (`self.K2_GetActorLocation`) (struct) (+ (`SceneComponent.K2_GetComponentScale` _returnvalue) (0.2 0.2 0.2)) false))
    (`KismetSystemLibrary.PrintString` (`KismetStringLibrary.Conv_VectorToString` (`SceneComponent.K2_GetComponentScale` _returnvalue_2)))))

(event `self.ProjectileMovement.OnProjectileStop`
  (params (ImpactResult :type "HitResult Structure (by ref)"))
  ;[1 1 1] 발사체 HIT 되었을 때, 생명주기, 이펙트 셋팅
  (`SceneComponent.SetHiddenInGame` (`self.Sphere`) true true)
  (`self.SetLifeSpan` 1.0)
  (`GameplayStatics.SpawnEmitterAttached` "/Game/JYJ/Blueprints/Skill/SkillBasic/P_AngelDissolve.P_AngelDissolve" (`self.Sphere`) "None" (0.0 0.0 0.0) (struct) (2.0 2.0 2.0)))

(event `self.ReceiveHit`
  (params (MyComp :type "PrimitiveComponent Object Reference") (Other :type "Actor Object Reference") (OtherComp :type "PrimitiveComponent Object Reference") (bSelfMoved :type Boolean) (HitLocation :type "Vector Structure") (HitNormal :type "Vector Structure") (NormalImpulse :type "Vector Structure") (Hit :type "HitResult Structure (by ref)"))
  ;[1 1 1] BOSS 액터 HIT 시, HP 차감 (추후, 데미지 UI 상 나오도록 수정 예정)
  (bind _asbp_boss (cast `/Game/KSH/Blueprints/BP_Boss` Other))
  (bind _resulthp (`/Game/KSH/Blueprints/BP_Boss.BossApplyDamage` _asbp_boss (`self.Damage`)))
  (set `/Game/KSH/Blueprints/BP_Boss.BossHP` _resulthp _asbp_boss)
  (`KismetSystemLibrary.PrintString` (`KismetStringLibrary.Conv_IntToString` (* (`self.Damage`) -1)) true true (struct :`R` 0.276042 :`G` 0.026942 :`A` 1.0)))

(fn `UserConstructionScript`)