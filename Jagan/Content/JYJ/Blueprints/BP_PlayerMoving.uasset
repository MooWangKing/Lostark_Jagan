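; BP_PlayerMoving is a player-controlled Blueprint that moves itself across the XY plane from axis input.
; BeginPlay calls EnableInput on player controller 0.
; The Horizonal axis offsets location along world Y and Vertical along world X, opposite to their axis comments.
; Each uses SetActorLocation with a fixed per-call step scaled by axis value, without sweep collision or delta-time scaling.
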(event `self.ReceiveBeginPlay`
  (`self.EnableInput` (`GameplayStatics.GetPlayerController` 0) null))

(event `InputAxis|Horizonal`
  (params (AxisValue :type "Float (single-precision)"))
  ;[1 1 1] X축 이동
  (`self.K2_SetActorLocation` (+ (* AxisValue (0.0 5.0 0.0)) (`self.K2_GetActorLocation`))))

(event `InputAxis|Vertical`
  (params (AxisValue :type "Float (single-precision)"))
  ;[1 1 1] Y축 이동
  (`self.K2_SetActorLocation` (+ (* AxisValue (5.0 0.0 0.0)) (`self.K2_GetActorLocation`))))

(fn `UserConstructionScript`)