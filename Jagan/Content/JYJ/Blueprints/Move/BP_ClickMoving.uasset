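; Player controller for right-click movement that walks the controlled pawn toward the mouse cursor while the MovingPlayer input is held.
; The input toggles a flag that Tick checks, skipping movement while BP_Player's hit or either skill-attack flag is set.
; Each moving tick traces under the cursor, calls SimpleMoveToLocation for points beyond a minimum distance, and spawns cursor and circle effects at any hit.
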(event `self.ReceiveTick`
  (params (DeltaSeconds :type "Float (single-precision)"))
  ;[1 1 1] IsClickRightMouse에 따라 마우스 커서로 위치 이동
  (bind _returnvalue (`GameplayStatics.GetActorOfClass` "/Game/JYJ/Blueprints/BP_Player.BP_Player_C"))
  (if (`/Game/JYJ/Blueprints/BP_Player.isHitted` _returnvalue)
    _
    (elif (`/Game/JYJ/Blueprints/BP_Player.isAttackedSkill1` _returnvalue)
      _
      (elif (`/Game/JYJ/Blueprints/BP_Player.isAttackedSkill2` _returnvalue)
        _
        (elif (`self.IsClickRightMouse`)
          (`self.MoveToMouseCursor`))))))

(event `InputAction|MovingPlayer`
  (params (Key :type "Key Structure"))
  ;[1 1 1] 우클릭 시, IsClickRightMouse 변수 값 변경
  (:`Pressed`
    (`self.InputRightMouseButtonPress`))
  (:`Released`
    (`self.InputRightMouseButtonRelease`)))

(fn `InputRightMouseButtonPress`
  (set `self.IsClickRightMouse` true))

(fn `InputRightMouseButtonRelease`
  (set `self.IsClickRightMouse` false))

(fn `MoveToMouseCursor`
  (bind (_hitresult _returnvalue) (`self.GetHitResultUnderCursorByChannel` self "TraceTypeQuery1" true))
  (bind (_bblockinghit _binitialoverlap _time _distance _location) (`GameplayStatics.BreakHitResult` _hitresult))
  (if _returnvalue
    (`self.SetNewDestination` _location)
    (`NiagaraFunctionLibrary.SpawnSystemAtLocation` (`self.FX_Cursor`) _location)
    (`NiagaraFunctionLibrary.SpawnSystemAtLocation` (`self.FX_Circle`) _location (struct) (3.0 3.0 3.0))))

(fn `SetNewDestination`
  (params (NewDirection :type "Vector Structure"))
  (if (> (`KismetMathLibrary.Vector_Distance` NewDirection (`self.K2_GetActorLocation` (`self.K2_GetPawn`))) 120.0)
    (`AIBlueprintHelperLibrary.SimpleMoveToLocation` self NewDirection)))

(fn `UserConstructionScript`)