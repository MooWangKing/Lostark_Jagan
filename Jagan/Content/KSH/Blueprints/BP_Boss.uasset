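; Boss actor that prototypes melee and ground-zone attacks, tagged by AttackType and played as animations on SMBOSS.
; BeginPlay resets Phase, prints BossHP, then after a delay starts a looping scratch with right-hand query collision enabled.
; Unwired chains hold an arm slam spawning a hit zone beneath the player, a stretch spawning two fixed-position zones, and a bite reusing the scratch animation.
; Collision-disable calls are also unwired.
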(event `self.ReceiveBeginPlay`
  (`|ExecutionSequence`
    (:`then_0`
      (set `self.Phase` 0))
    (:`then_1`
      (`KismetSystemLibrary.PrintString` (`KismetStringLibrary.Conv_IntToString` (`self.BossHP`)))
      (`KismetSystemLibrary.Delay` 2.0)
      ;[1 1 1] 할퀴기 공격 실행 -> 손에 공격 판정 O -> 끝나면 판정 X
      (set `self.AttackType` 1)
      (`|ExecutionSequence`
        (:`then_0`
          (`PrimitiveComponent.SetCollisionEnabled` (`self.RightHandCollision`) "QueryOnly"))
        (:`then_1`
          (`SkeletalMeshComponent.PlayAnimation` (`self.SM_BOSS`) "/Game/KSH/Animations/Anim/A_ScratchAnim.A_ScratchAnim" true))))))

(fn `UserConstructionScript`)