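; BP_WallController is an interaction point that lowers the level's BP_Wall once the boss's HP reaches zero.
; Its Range overlap shows or hides a text widget and image for BP_Player, and a separate event enables that range's collision.
; OpenWall moves the wall down through a Delay loop capped by DoN at 20 steps.
; As written, its constant 0 >= 20 check never disables the wall's collision.
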(event `self.ReceiveBeginPlay`
  (`|ExecutionSequence`
    (:`then_0`
      (bind _returnvalue (`GameplayStatics.GetActorOfClass` "/Game/KSH/Blueprints/BP_Boss.BP_Boss_C"))
      (set `self.BPBoss` _returnvalue))
    (:`then_1`
      (bind _returnvalue_2 (`GameplayStatics.GetActorOfClass` "/Game/KSH/Blueprints/BP_Wall.BP_Wall_C"))
      (set `self.Wall` _returnvalue_2))
    (:`then_2`
      (`SceneComponent.SetVisibility` (`self.WidgetWorkText`) false false)
      (`SceneComponent.SetVisibility` (`self.WorkImage`) false false))))

(event `self.ReceiveTick`
  (params (DeltaSeconds :type "Float (single-precision)")))

(event `OpenWall`
  (bind _wall (`self.Wall`))
  ;[1 1 1] OpenWall
  (if (<= (`/Game/KSH/Blueprints/BP_Boss.BossHP` (`self.BPBoss`)) 0)
    (`/Engine/EditorBlueprintResources/StandardMacros.Do N` 20 :!label _label
      (:`Exit`
        (`self.K2_SetActorLocation` _wall (+ (`self.K2_GetActorLocation` _wall) (* (`GameplayStatics.GetWorldDeltaSeconds`) (0.0 0.0 -1.5) (`self.Speed`))) false false)
        (`KismetSystemLibrary.PrintString` "\"Open Wall\"")
        (`KismetSystemLibrary.Delay` 0.2)
        (if (>= 0 20)
          (`PrimitiveComponent.SetCollisionEnabled` (`/Game/KSH/Blueprints/BP_Wall.Cube` (`self.Wall`)) "NoCollision")
          (else
            (goto _label)))))
    (else
      (`KismetSystemLibrary.PrintString` "\"보스 HP가 0이 아님\""))))

(event `self.Range.OnComponentBeginOverlap`
  (params (OverlappedComponent :type "PrimitiveComponent Object Reference") (OtherActor :type "Actor Object Reference") (OtherComp :type "PrimitiveComponent Object Reference") (OtherBodyIndex :type Integer) (bFromSweep :type Boolean) (SweepResult :type "HitResult Structure (by ref)"))
  ;[1 1 1] 근처에 도달하면 Visible하게 / 나가면 안보이게
  (`self.WorkTextAndImageVisiblilty` true OtherActor))

(event `self.Range.OnComponentEndOverlap`
  (params (OverlappedComponent :type "PrimitiveComponent Object Reference") (OtherActor :type "Actor Object Reference") (OtherComp :type "PrimitiveComponent Object Reference") (OtherBodyIndex :type Integer))
  ;[1 1 1] 근처에 도달하면 Visible하게 / 나가면 안보이게
  (`self.WorkTextAndImageVisiblilty` false OtherActor))

(event `WorkTextAndImageVisiblilty`
  (params (IsCollsion :type Boolean) (Player :type "Actor Object Reference"))
  ;[1 1 1] 안보이게 하는 이벤트 작성
  (cast `/Game/JYJ/Blueprints/BP_Player` Player)
  (`SceneComponent.SetVisibility` (`self.WidgetWorkText`) IsCollsion false)
  (`SceneComponent.SetVisibility` (`self.WorkImage`) IsCollsion false))

(event `WallControllerCollsionEnabled`
  ;[1 1 1] 콜리전 가능하게
  (`PrimitiveComponent.SetCollisionEnabled` (`self.Range`) "QueryAndPhysics"))

(event `self.ReceiveActorBeginOverlap`
  (params (OtherActor :type "Actor Object Reference")))

(fn `UserConstructionScript`)