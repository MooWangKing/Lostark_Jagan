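; BP_FireSpawnFloor is a fire area hazard actor with a falling Sphere that burns the player on overlap.
; Tick moves the Sphere straight down by Speed without sweep, and actor overlap casts to BP_Player to apply damage over time.
; A delayed sequence that enables Plane collision, spawns a burning emitter and destroys the actor is disconnected, so it never runs.
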(event `self.ReceiveBeginPlay`)

(event `self.ReceiveTick`
  (params (DeltaSeconds :type "Float (single-precision)"))
  (bind _sphere (`self.Sphere`))
  ;[1 1 1] 이펙트 아래로 떨어지게
  (`SceneComponent.K2_SetWorldLocation` _sphere (+ (`SceneComponent.K2_GetComponentLocation` _sphere) (* (`GameplayStatics.GetWorldDeltaSeconds`) (0.0 0.0 -1.0) (`self.Speed`))) false false))

(event `self.ReceiveActorBeginOverlap`
  (params (OtherActor :type "Actor Object Reference"))
  ;[1 1 1] 플레이어 공격 처리
  (bind _asbp_player (cast `/Game/JYJ/Blueprints/BP_Player` OtherActor))
  (`/Game/JYJ/Blueprints/BP_Player.PlayerApplyDotDamageEvent` _asbp_player 10 2))

(fn `UserConstructionScript`)