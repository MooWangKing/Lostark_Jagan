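; BP_PlayerTest is a test player for exercising boss fight and wall interaction mechanics.
; Tick moves it along its forward and right vectors from axis input, setting location without sweep, and overlaps print the touched actor's name.
; It caches BP_Boss on BeginPlay for debug inputs that zero boss HP or switch phase.
; G sphere-checks nearby BP_WallController actors and calls OpenWall on them.
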(event `self.ReceiveTick`
  (params (DeltaSeconds :type "Float (single-precision)"))
  (`self.Translate` (`self.Speed`) (`KismetMathLibrary.Normal` (+ (* (`self.GetInputAxisValue`) (`self.GetActorRightVector`)) (* (`self.GetInputAxisValue`) (`self.GetActorForwardVector`))))))

(event `self.ReceiveActorBeginOverlap`
  (params (OtherActor :type "Actor Object Reference"))
  ;[1 1 1] 장판 맞으면 맞은 장판 이름 화면에 표시
  (`KismetSystemLibrary.PrintString` (`KismetSystemLibrary.GetDisplayName` OtherActor)))

(event `self.ReceiveBeginPlay`
  ;[1 1 1] HP 0 Test
  (bind _returnvalue (`GameplayStatics.GetActorOfClass` "/Game/KSH/Blueprints/BP_Boss.BP_Boss_C"))
  (bind _asbp_boss (cast `/Game/KSH/Blueprints/BP_Boss` _returnvalue))
  (set `self.BPBoss` _asbp_boss))

(event `InputAction|BossHPDecreaseTest`
  (params (Key :type "Key Structure"))
  (bind _bpboss (`self.BPBoss`))
  ;[1 1 1] HP 0 Test
  (:`Pressed`
    (set `/Game/KSH/Blueprints/BP_Boss.BossHP` 0 _bpboss)
    (`KismetSystemLibrary.PrintString` (`KismetStringLibrary.Conv_IntToString` (`/Game/KSH/Blueprints/BP_Boss.BossHP` _bpboss)))))

(event `Key|G`
  (params (Key :type "Key Structure"))
  ;[1 1 1] 범위에 있으면 상호작용 가능
  (:`Pressed`
    (bind (_outactors _returnvalue) (`KismetSystemLibrary.SphereOverlapActors` (`self.K2_GetActorLocation`) 200.0 (`|MakeArray` "ObjectTypeQuery2" :!type "EObjectTypeQuery Enum") "/Game/KSH/Blueprints/BP_WallController.BP_WallController_C"))
    (if _returnvalue
      (for _array_element _outactors
        (bind _asbp_wall_controller (cast `/Game/KSH/Blueprints/BP_WallController` _array_element))
        (`/Game/KSH/Blueprints/BP_WallController.OpenWall` _asbp_wall_controller)))))

(event `Key|One`
  (params (Key :type "Key Structure"))
  ;[1 1 1] 페이즈 변경
  (:`Pressed`
    (set `/Game/KSH/Blueprints/BP_Boss.Phase` 1 (`self.BPBoss`))))

(event `Key|Zero`
  (params (Key :type "Key Structure"))
  ;[1 1 1] 페이즈 변경
  (:`Pressed`
    (set `/Game/KSH/Blueprints/BP_Boss.Phase` 0 (`self.BPBoss`))))

(fn `Translate`
  (params (Speed :type "Float (double-precision)") (Direction :type "Vector Structure"))
  (`self.K2_SetActorLocation` (+ (`self.K2_GetActorLocation`) (* Speed Direction (`GameplayStatics.GetWorldDeltaSeconds`)))))

(fn `UserConstructionScript`)