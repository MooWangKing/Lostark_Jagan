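; BP_DamageTextBoss is a floating damage number actor, named for use with bosses, that animates and then removes itself.
; SetDamageText writes the damage value to its TextRender component as an integer.
; On BeginPlay a timeline vector track drives the text, with Z as height offset from the spawn location and Y as X/Y text scale.
; The actor destroys itself when the timeline finishes.
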(event `self.ReceiveBeginPlay`
  (bind _textrender (`self.TextRender`))
  (set `self.StartPos` (`self.K2_GetActorLocation`))
  (bind (_direction _newtrack_1) (`Timeline|DamageTextTimeline`)
    (:`Update`
      (bind _y (.y _newtrack_1))
      (`SceneComponent.K2_SetWorldLocation` (`self.TextRender`) (+ (`self.StartPos`) (`KismetMathLibrary.MakeVector` 0.0 0.0 (.z _newtrack_1))) false false)
      (`TextRenderComponent.SetXScale` _textrender _y)
      (`TextRenderComponent.SetYScale` _textrender _y))
    (:`Finished`
      (`self.K2_DestroyActor`))))

(fn `SetDamageText`
  (params (Damage :type Integer))
  (`TextRenderComponent.K2_SetText` (`self.TextRender`) (`KismetTextLibrary.Conv_IntToText` Damage)))

(fn `UserConstructionScript`)